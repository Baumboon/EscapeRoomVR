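; VR elevator button that represents one level, built on a parent pressable button.
; On BeginPlay it reads its LevelInfo status to set color and interactivity: grey and disabled, red when available, green when finished.
; A button with no level path prints an on-screen warning instead.
; A full press prints the button's name and broadcasts OnClick with the LevelInfo, leaving any level travel to listeners.
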(event EventBeginPlay
  (|CallParentFunction)
  (if (Utilities|Name|NotEqual(Name) (.levelpath (Variables|Default|GetLevelInfo)) "None")
    (switch Utilities|FlowControl|Switch|SwitchonELevelStatus (.status (Variables|Default|GetLevelInfo))
      (:NewEnumerator2
        (CallFunction|SetBaseColor "(R=0.333333,G=0.333333,B=0.333333,A=1.000000)")
        (CallFunction|ToggleEnable false))
      (:NewEnumerator0
        (CallFunction|SetBaseColor "(R=0.947917,G=0.029125,B=0.019696,A=1.000000)")
        (CallFunction|ToggleEnable true :!label _label))
      (:NewEnumerator1
        (CallFunction|SetBaseColor "(R=0.360883,G=1.000000,B=0.102896,A=1.000000)")
        (goto _label)))
    (else
      (Development|PrintString (Utilities|String|Append (Utilities|GetDisplayName self) "has no level selected") true true "(R=1.000000,G=0.022377,B=0.000000,A=1.000000)"))))

(event EventFullyPressed
  (Development|PrintString (Utilities|GetDisplayName self))
  (Default|CallOnClick (Variables|Default|GetLevelInfo)))

(fn ConstructionScript
  (|CallParentFunction))