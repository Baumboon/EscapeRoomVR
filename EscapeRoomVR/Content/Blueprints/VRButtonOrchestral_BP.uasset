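; VR button Blueprint, named for an orchestral feature, that shows correct and wrong feedback through its base color.
; It extends a parent button, with events that tint it green for correct, red for wrong, or gray on reset.
; Reset also switches off glowing, and runs after the parent's end-of-input handling when the button is enabled.
; The calls that would switch glowing on are left unconnected.
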(event Custom|Reset
  (CallFunction|SetBaseColor "(R=0.254902,G=0.254902,B=0.254902,A=1.000000)")
  (CallFunction|ToggleGlowing false))

(event Custom|ShowWrong
  (CallFunction|SetBaseColor "(R=0.489583,G=0.029711,B=0.000000,A=1.000000)"))

(event Custom|ShowCorrect
  (CallFunction|SetBaseColor "(R=0.009958,G=0.364583,B=0.000000,A=1.000000)"))

(event EventBeginPlay
  (|CallParentFunction) ; This node is disabled and will not be called.\nDrag off pins to build functionality.
)

(event Collision|EventActorBeginOverlap
  (params (OtherActor :type Actor%20Object%20Reference)))

(event EventTick
  (params (DeltaSeconds :type Float%20%28single-precision%29))
  (|CallParentFunction DeltaSeconds) ; This node is disabled and will not be called.\nDrag off pins to build functionality.
)

(event EventOnEndInput
  (|CallParentFunction)
  (if (Variables|Default|GetbEnabled)
    (CallFunction|Reset)))

(fn ConstructionScript
  (|CallParentFunction))