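; Game mode for an escape game that manages level streaming and progression around an elevator hub.
; On BeginPlay it loads the game through the game instance, respawns elevator buttons, streams the first level and opens the elevator.
; StreamLevel replaces the active streamed level, and IsLoaded compares level numbers against it.
; FinishLevel updates the current and next level statuses in the game instance, then refreshes and reopens the elevator.
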(event Custom|StreamLevel
  (params (Level :type Level%20Info%20Structure))
  (if (Utilities|Name|Equal(Name) (.LevelPath (Utilities|Struct|BreakLevelInfo (Variables|Default|GetActiveLevel))) "None")
    _
    (else
      (Game|UnloadStreamLevel(byName) (.LevelPath (Utilities|Struct|BreakLevelInfo (Variables|Default|GetActiveLevel))) true)))
  (bind _output_get (Variables|Default|SetActiveLevel Level))
  (Game|LoadStreamLevel(byName) (.levelpath _output_get) true))

(event Custom|FinishLevel
  (bind _activelevel (Variables|Default|GetActiveLevel))
  (bind _returnvalue (+ (.number _activelevel) 1))
  (bind _asescape_gi_bp (Utilities|Casting|CastToEscapeGI_BP (Game|GetGameInstance)))
  (Utilities|FlowControl|Sequence
    (:then_0
      (bind _structout (Utilities|Struct|SetmembersinLevelInfo (Utilities|Array|Get(acopy) (Variables|/Game/Blueprints/EscapeGI_BP.EscapeGI_BP_C|GetLevelStatus _asescape_gi_bp) (.number _activelevel)) "NewEnumerator1"))
      (Utilities|Array|SetArrayElem (Variables|/Game/Blueprints/EscapeGI_BP.EscapeGI_BP_C|GetLevelStatus _asescape_gi_bp) (.number _activelevel) _structout))
    (:then_1
      (if (> (Utilities|Array|Length (Variables|/Game/Blueprints/EscapeGI_BP.EscapeGI_BP_C|GetLevelStatus _asescape_gi_bp)) _returnvalue)
        (bind _structout_2 (Utilities|Struct|SetmembersinLevelInfo (Utilities|Array|Get(acopy) (Variables|/Game/Blueprints/EscapeGI_BP.EscapeGI_BP_C|GetLevelStatus _asescape_gi_bp) _returnvalue) "NewEnumerator0"))
        (Utilities|Array|SetArrayElem (Variables|/Game/Blueprints/EscapeGI_BP.EscapeGI_BP_C|GetLevelStatus _asescape_gi_bp) _returnvalue _structout_2)))
    (:then_2
      (bind _returnvalue_2 (Actor|GetActorOfClass "/Game/Blueprints/Elevator.Elevator_C"))
      (Default|RespawnButtons _returnvalue_2)
      (Default|Open _returnvalue_2))))

(event EventBeginPlay
  (bind _asescape_gi_bp (Utilities|Casting|CastToEscapeGI_BP (Game|GetGameInstance)))
  (Default|LoadGame _asescape_gi_bp)
  (bind _returnvalue (Actor|GetActorOfClass "/Game/Blueprints/Elevator.Elevator_C"))
  (Default|RespawnButtons _returnvalue)
  (CallFunction|StreamLevel (Utilities|Array|Get(acopy) (Variables|/Game/Blueprints/EscapeGI_BP.EscapeGI_BP_C|GetLevelStatus _asescape_gi_bp)))
  (Default|Open _returnvalue))

(fn ConstructionScript)

(fn IsLoaded
  (params (Level :type Level%20Info%20Structure))
  (return (== (.number Level) (.number (Variables|Default|GetActiveLevel)))))