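; Laser barrier actor that detects when something breaks the beam between its Sender and Receiver components.
; Each tick it line traces between the two against world, pawn and physics body objects, drawing the trace for one frame as a debug line.
; The beam counts as interrupted when the hit component is not the Receiver.
; It broadcasts OnLaserInterrupted only when that state changes.
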(event EventTick
  (params (DeltaSeconds :type Float%20%28single-precision%29))
  (bind _outhit (Collision|LineTraceForObjects (Transformation|GetWorldLocation (Variables|Default|GetSender)) (Transformation|GetWorldLocation (Variables|Default|GetReceiver)) (Utilities|Array|MakeArray "ObjectTypeQuery1" "ObjectTypeQuery2" "ObjectTypeQuery3" "ObjectTypeQuery4") false 0 "ForOneFrame" false "(R=0.594295,G=5.000000,B=0.000000,A=1.000000)" "(R=5.000000,G=0.240031,B=0.000000,A=1.000000)"))
  (if (Math|Boolean|NotEqual(Boolean) (Variables|Default|GetbInterrupted) (!= (.HitComponent (Collision|BreakHitResult _outhit)) (Variables|Default|GetReceiver)))
    (bind _output_get (Variables|Default|SetbInterrupted (!= (.HitComponent (Collision|BreakHitResult _outhit)) (Variables|Default|GetReceiver))))
    (Default|CallOnLaserInterrupted self _output_get)))

(fn ConstructionScript)