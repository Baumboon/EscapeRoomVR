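; VR button Blueprint, named as a laser button, that finishes the level in the escape game when fully pressed.
; On a change of enabled state it calls the parent logic and sets the base color to green when enabled or red when disabled.
; A full press runs the parent handler, then casts the game mode to EscapeGM_BP and calls FinishLevel.
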(event Custom|ToggleEnable
  (params (bEnabled :type Boolean))
  (if (Math|Boolean|NotEqual(Boolean) bEnabled (Variables|Default|GetbEnabled))
    (|CallParentFunction bEnabled)
    (if bEnabled
      (CallFunction|SetBaseColor "(R=0.570726,G=0.812500,B=0.199375,A=1.000000)")
      (else
        (CallFunction|SetBaseColor "(R=0.906250,G=0.000000,B=0.006923,A=1.000000)")))))

(event EventFullyPressed
  (|CallParentFunction)
  (if true
    (bind _asescape_gm_bp (Utilities|Casting|CastToEscapeGM_BP (Game|GetGameMode)))
    (Default|FinishLevel _asescape_gm_bp)))

(fn ConstructionScript
  (|CallParentFunction))