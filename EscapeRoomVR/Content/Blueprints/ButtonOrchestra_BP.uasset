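; VR memory puzzle actor with nine orchestral buttons, where the player repeats a randomly generated four-button sequence.
; Overlap by the motion controller pawn's sphere generates a sequence and plays it as timer-driven glows, which any press interrupts.
; Press events validate each step in order; mistakes flag all buttons wrong and regenerate the puzzle after release.
; Success disables the buttons and raises the actor on a timeline.
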(event OnComponentBeginOverlap(Box)
  (params (OverlappedComponent :type Primitive%20Component%20Object%20Reference) (OtherActor :type Actor%20Object%20Reference) (OtherComp :type Primitive%20Component%20Object%20Reference) (OtherBodyIndex :type Integer) (bFromSweep :type Boolean) (SweepResult :type Hit%20Result%20Structure%20%28by%20ref%29))
  (Development|PrintString (Utilities|GetDisplayName OtherComp))
  (bind _asmotion_controller_pawn (Utilities|Casting|CastToMotionControllerPawn OtherActor))
  (if (and (== (Variables|/Game/EpicTemplates/VRTemplate/Blueprints/MotionControllerPawn.MotionControllerPawn_C|GetSphere _asmotion_controller_pawn) OtherComp) (not (Variables|Default|GetbVisualizingOrder)))
    (CallFunction|ResetGrid)))

(event Custom|GenerateButtonOrder
  (params (Count :type Integer))
  (bind _allbuttons (Variables|Default|GetAllButtons))
  (Utilities|Array|Clear (Variables|Default|GetSequenceButtons))
  (for _index (range 0 (- Count 1))
    (Utilities|Array|Add (Variables|Default|GetSequenceButtons) (Utilities|Array|Get(acopy) _allbuttons (Math|Random|RandomIntegerinRange 0 (- (Utilities|Array|Length _allbuttons) 1))))))

(event Custom|ResetGrid
  (Default|Reset (Variables|Default|GetAllButtons))
  (CallFunction|GenerateButtonOrder 4)
  (CallFunction|StartOrderVisualization)
  (Variables|Default|SetButtonIndex 0))

(event Custom|HandleButtonPressed
  (params (Button :type VR%20Button%20Base%20BP%20Object%20Reference))
  (Utilities|FlowControl|Sequence
    (:then_0
      (if (Variables|Default|GetbVisualizingOrder)
        (CallFunction|AbortOrderVisualization)))
    (:then_1
      (if (== Button (Utilities|Array|Get(acopy) (Variables|Default|GetSequenceButtons) (Variables|Default|GetButtonIndex)))
        (Default|ShowCorrect (Utilities|Array|Get(acopy) (Variables|Default|GetSequenceButtons) (Variables|Default|GetButtonIndex)))
        (Variables|Default|SetButtonIndex (+ (Variables|Default|GetButtonIndex) 1))
        (if (>= (Variables|Default|GetButtonIndex) (Utilities|Array|Length (Variables|Default|GetSequenceButtons)))
          (CallFunction|CompleteInput))
        (else
          (CallFunction|AbortInput))))))

(event Custom|AbortInput
  (for _array_element (Variables|Default|GetAllButtons)
    (Default|ShowWrong _array_element)
    (Variables|Default|SetButtonIndex -1)))

(event Custom|HighlightButton
  (bind _sequencebuttons (Variables|Default|GetSequenceButtons))
  (if (Utilities|Array|IsValidIndex _sequencebuttons (Variables|Default|GetEmissionIndex))
    (Default|ToggleGlowing (Utilities|Array|Get(acopy) _sequencebuttons (Variables|Default|GetEmissionIndex)) true)
    (Utilities|FlowControl|Delay 1.0)
    (Default|ToggleGlowing (Utilities|Array|Get(acopy) _sequencebuttons (Variables|Default|GetEmissionIndex)) false)
    (Variables|Default|SetEmissionIndex (+ (Variables|Default|GetEmissionIndex) 1))
    (if (>= (Variables|Default|GetEmissionIndex) (Utilities|Array|Length (Variables|Default|GetSequenceButtons)))
      (CallFunction|AbortOrderVisualization))))

(event Custom|AbortOrderVisualization
  (bind _sequencebuttons (Variables|Default|GetSequenceButtons))
  (if (Utilities|Array|IsValidIndex _sequencebuttons (Variables|Default|GetEmissionIndex))
    (Default|ToggleGlowing (Utilities|Array|Get(acopy) _sequencebuttons (Variables|Default|GetEmissionIndex)) false))
  (Utilities|Time|ClearandInvalidateTimerbyHandle (Variables|Default|GetEmissionTimer))
  (Variables|Default|SetEmissionIndex 0)
  (Variables|Default|SetbVisualizingOrder false))

(event Custom|StartOrderVisualization
  (Variables|Default|SetbVisualizingOrder true)
  (CallFunction|HighlightButton)
  (bind _returnvalue (Utilities|Time|SetTimerbyEvent (EventDispatchers|CreateEvent :!event Custom|HighlightButton) 1.5 true))
  (Variables|Default|SetEmissionTimer _returnvalue))

(event Custom|CompleteInput
  (for _array_element (Variables|Default|GetAllButtons)
    (Default|ShowCorrect _array_element)
    (Default|ToggleEnable _array_element false)
    (Variables|Default|SetButtonIndex -1)
    (Variables|Default|SetbCompleted true)
    (bind _newtrack_0 (Timeline|MoveTimeline Play)
      (:Update
        (Transformation|SetActorLocation (+ (Variables|Default|GetInitialLocation) (* "0,0.000000,250.000000" _newtrack_0)) false false)))))

(event Custom|HandleButtonReleased
  (params (Button :type VR%20Button%20Base%20BP%20Object%20Reference))
  (if (and (< (Variables|Default|GetButtonIndex) 0) (not (Variables|Default|GetbCompleted)))
    (Default|Reset (Variables|Default|GetAllButtons))
    (Utilities|FlowControl|Delay 0.5)
    (CallFunction|ResetGrid)))

(event EventBeginPlay
  (Variables|Default|SetInitialLocation (Transformation|GetActorLocation))
  (bind _output_get (Variables|Default|SetAllButtons (Utilities|Array|MakeArray (.AsVRButton%20Orchestral%20BP (Utilities|Casting|CastToVRButtonOrchestral_BP (Variables|/Script/Engine.ChildActorComponent|GetChildActor (Variables|Default|GetChildActor)))) (.AsVRButton%20Orchestral%20BP (Utilities|Casting|CastToVRButtonOrchestral_BP (Variables|/Script/Engine.ChildActorComponent|GetChildActor (Variables|Default|GetChildActor1)))) (.AsVRButton%20Orchestral%20BP (Utilities|Casting|CastToVRButtonOrchestral_BP (Variables|/Script/Engine.ChildActorComponent|GetChildActor (Variables|Default|GetChildActor2)))) (.AsVRButton%20Orchestral%20BP (Utilities|Casting|CastToVRButtonOrchestral_BP (Variables|/Script/Engine.ChildActorComponent|GetChildActor (Variables|Default|GetChildActor3)))) (.AsVRButton%20Orchestral%20BP (Utilities|Casting|CastToVRButtonOrchestral_BP (Variables|/Script/Engine.ChildActorComponent|GetChildActor (Variables|Default|GetChildActor4)))) (.AsVRButton%20Orchestral%20BP (Utilities|Casting|CastToVRButtonOrchestral_BP (Variables|/Script/Engine.ChildActorComponent|GetChildActor (Variables|Default|GetChildActor5)))) (.AsVRButton%20Orchestral%20BP (Utilities|Casting|CastToVRButtonOrchestral_BP (Variables|/Script/Engine.ChildActorComponent|GetChildActor (Variables|Default|GetChildActor6)))) (.AsVRButton%20Orchestral%20BP (Utilities|Casting|CastToVRButtonOrchestral_BP (Variables|/Script/Engine.ChildActorComponent|GetChildActor (Variables|Default|GetChildActor7)))) (.AsVRButton%20Orchestral%20BP (Utilities|Casting|CastToVRButtonOrchestral_BP (Variables|/Script/Engine.ChildActorComponent|GetChildActor (Variables|Default|GetChildActor8)))))))
  (for _array_element _output_get
    (EventDispatchers|BindEventtoOnButtonFullyPressed _array_element (EventDispatchers|CreateEvent :!event Custom|HandleButtonPressed))
    (EventDispatchers|AssignOnButtonReleased _array_element (EventDispatchers|CreateEvent :!event Custom|HandleButtonReleased))))

(fn ConstructionScript)