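; Game instance Blueprint for the Escape game that holds per-level status and persists it through an EscapeSaveGame_BP save slot.
; LoadGame copies the saved level list into LevelStatus, or calls CreateGame when the load fails or the list length differs from DefaultLevels.
; CreateGame resets to the defaults in a new save object, so a changed level count discards old progress.
; SaveGame writes LevelStatus back to the slot.
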(event Custom|LoadGame
  (bind _returnvalue (SaveGame|LoadGamefromSlot (Variables|Default|GetSlotName)))
  (bind _asescape_save_game_bp (Utilities|Casting|CastToEscapeSaveGame_BP _returnvalue)
    (:then
      (bind _output_get (Variables|Default|SetSaveGameInstance _asescape_save_game_bp))
      (bind _output_get_2 (Variables|Default|SetLevelStatus (Variables|/Game/Blueprints/EscapeSaveGame_BP.EscapeSaveGame_BP_C|GetLevelList _output_get)))
      (if (!= (Utilities|Array|Length _output_get_2) (Utilities|Array|Length (Variables|Default|GetDefaultLevels)))
        (CallFunction|CreateGame)))
    (:CastFailed
      (CallFunction|CreateGame))))

(event Custom|SaveGame
  (bind _savegameinstance (Variables|Default|GetSaveGameInstance))
  (Variables|/Game/Blueprints/EscapeSaveGame_BP.EscapeSaveGame_BP_C|SetLevelList _savegameinstance (Variables|Default|GetLevelStatus))
  (SaveGame|SaveGametoSlot _savegameinstance (Variables|Default|GetSlotName)))

(event Custom|CreateGame
  (Variables|Default|SetLevelStatus (Variables|Default|GetDefaultLevels))
  (bind _returnvalue (SaveGame|CreateSaveGameObject "/Game/Blueprints/EscapeSaveGame_BP.EscapeSaveGame_BP_C"))
  (Variables|Default|SetSaveGameInstance _returnvalue)
  (CallFunction|SaveGame))