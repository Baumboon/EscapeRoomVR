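; VR elevator for an escape game that hides level streaming behind closing doors.
; One timeline slides four door components, playing to close and reversing to open; doors also close when the MotionControllerPawn exits the box.
; RespawnButtons builds a three-column grid of clickable buttons from the game instance's LevelStatus.
; HandleButtonClicked closes the doors for an unloaded level, waits, asks EscapeGM_BP to stream it, then reopens.
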(event OnComponentEndOverlap(Box)
  (params (OverlappedComponent :type Primitive%20Component%20Object%20Reference) (OtherActor :type Actor%20Object%20Reference) (OtherComp :type Primitive%20Component%20Object%20Reference) (OtherBodyIndex :type Integer))
  (Utilities|Casting|CastToMotionControllerPawn OtherActor)
  (CallFunction|Close))

(event Custom|Open
  (bind _newtrack_0 (Timeline|Timeline_0 Reverse)
    (:Update
      (Transformation|SetRelativeLocation (Variables|Default|GetScene1) (Math|Vector|MakeVector (* _newtrack_0 (Variables|Default|GetDoorSpeed)) 0.0 0.0) false false)
      (Transformation|SetRelativeLocation (Variables|Default|GetScene3) (Math|Vector|MakeVector (* _newtrack_0 (Variables|Default|GetDoorSpeed)) 0.0 0.0) false false)
      (Transformation|SetRelativeLocation (Variables|Default|GetDoorInner) (Math|Vector|MakeVector (* _newtrack_0 (Variables|Default|GetDoorSpeed)) 0.0 0.0) false false)
      (Transformation|SetRelativeLocation (Variables|Default|GetDoorInner1) (Math|Vector|MakeVector (* _newtrack_0 (Variables|Default|GetDoorSpeed)) 0.0 0.0) false false))))

(event Custom|Close
  (bind _newtrack_0 (Timeline|Timeline_0 Play)
    (:Update
      (Transformation|SetRelativeLocation (Variables|Default|GetScene1) (Math|Vector|MakeVector (* _newtrack_0 (Variables|Default|GetDoorSpeed)) 0.0 0.0) false false)
      (Transformation|SetRelativeLocation (Variables|Default|GetScene3) (Math|Vector|MakeVector (* _newtrack_0 (Variables|Default|GetDoorSpeed)) 0.0 0.0) false false)
      (Transformation|SetRelativeLocation (Variables|Default|GetDoorInner) (Math|Vector|MakeVector (* _newtrack_0 (Variables|Default|GetDoorSpeed)) 0.0 0.0) false false)
      (Transformation|SetRelativeLocation (Variables|Default|GetDoorInner1) (Math|Vector|MakeVector (* _newtrack_0 (Variables|Default|GetDoorSpeed)) 0.0 0.0) false false))))

(event Custom|HandleButtonClicked
  (params (LevelInfo :type Level%20Info%20Structure))
  (bind _asescape_gm_bp (Utilities|Casting|CastToEscapeGM_BP (Game|GetGameMode)))
  (bind _newparam1 (Default|IsLoaded _asescape_gm_bp LevelInfo))
  (if (not _newparam1)
    (CallFunction|Close)
    (Development|PrintString "post close")
    (Utilities|FlowControl|Delay 2.0)
    (bind _asescape_gm_bp_2 (Utilities|Casting|CastToEscapeGM_BP (Game|GetGameMode)))
    (Development|PrintString "pre load")
    (Default|StreamLevel _asescape_gm_bp_2 LevelInfo)
    (Development|PrintString "post load")
    (CallFunction|Open)
    (Development|PrintString "post open")))

(event Collision|EventActorBeginOverlap
  (params (OtherActor :type Actor%20Object%20Reference)))

(event EventTick
  (params (DeltaSeconds :type Float%20%28single-precision%29)))

(fn ConstructionScript)

(fn RespawnButtons
  (bind _buttongrid (Variables|Default|GetButtonGrid))
  (Actor|DestroyActor _buttongrid)
  (Utilities|Array|Clear _buttongrid)
  (bind _asescape_gi_bp (Utilities|Casting|CastToEscapeGI_BP (Game|GetGameInstance)))
  (for (_array_element _array_index) (Variables|/Game/Blueprints/EscapeGI_BP.EscapeGI_BP_C|GetLevelStatus _asescape_gi_bp)
    (bind _returnvalue (Game|SpawnActorfromClass "/Game/Blueprints/VRButtonElevator_BP.VRButtonElevator_BP_C" (CallFunction|CalcButtonTransform _array_index) "Undefined" 0 _array_element 0))
    (Utilities|Array|Add (Variables|Default|GetButtonGrid) _returnvalue)
    (Transformation|AttachComponentToComponent _returnvalue (Variables|Default|GetButtonSocket) "None" "KeepRelative" "KeepRelative" "KeepRelative" true)
    (EventDispatchers|BindEventtoOnClick _returnvalue (EventDispatchers|CreateEvent :!event Custom|HandleButtonClicked))
    (Default|Init _returnvalue)))

(fn CalcButtonTransform
  (params (Index :type Integer))
  (return (Math|Transform|MakeTransform (Math|Vector|MakeVector (* (Math|Integer|%(Integer) Index 3) 1e+01) (* (/ Index 3) 1e+01) 0.0) "0, 0, 0" (Math|Conversions|ToVector(Float) 0.25))))