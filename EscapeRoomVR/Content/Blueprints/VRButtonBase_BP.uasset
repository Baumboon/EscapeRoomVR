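; Base VR push button that a BP_MotionController physically pushes along its up axis, firing an OnButtonFullyPressed event at maximum travel when enabled.
; On overlap it tracks the controller, projecting its movement onto the button's up vector to offset the mesh each Tick.
; A full press stops tracking and raises glow on a dynamic material created in the construction script.
; Ending overlap optionally interpolates it back to rest, then resets the glow.
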(event OnComponentBeginOverlap(VR_Button)
  (params (OverlappedComponent :type Primitive%20Component%20Object%20Reference) (OtherActor :type Actor%20Object%20Reference) (OtherComp :type Primitive%20Component%20Object%20Reference) (OtherBodyIndex :type Integer) (bFromSweep :type Boolean) (SweepResult :type Hit%20Result%20Structure%20%28by%20ref%29))
  (Development|PrintString "begin")
  (if (and (not (Variables|Default|GetbIsReturning)) (not (Variables|Default|GetbIsTracking)))
    (bind _asbp_motion_controller (Utilities|Casting|CastToBP_MotionController OtherActor))
    (Variables|Default|SetTracking%20MC (Variables|/Game/EpicTemplates/VRTemplate/Blueprints/BP_MotionController.BP_MotionController_C|GetMotionController _asbp_motion_controller))
    (Variables|Default|SetbIsTracking true)
    (Variables|Default|SetMC%20intial%20Location (Transformation|GetWorldLocation (Variables|Default|GetTracking%20MC)))
    (bind _output_get (Variables|Default|SetButton%20initial%20Location (Transformation|GetWorldLocation (Variables|Default|GetVR_Button))))
    (Development|PrintString (Utilities|String|Append "init " (Utilities|String|ToString(Vector) _output_get)))))

(event OnComponentEndOverlap(VR_Button)
  (params (OverlappedComponent :type Primitive%20Component%20Object%20Reference) (OtherActor :type Actor%20Object%20Reference) (OtherComp :type Primitive%20Component%20Object%20Reference) (OtherBodyIndex :type Integer))
  (Development|PrintString "end")
  (bind _asbp_motion_controller (Utilities|Casting|CastToBP_MotionController OtherActor))
  (if (== (Variables|/Game/EpicTemplates/VRTemplate/Blueprints/BP_MotionController.BP_MotionController_C|GetMotionController _asbp_motion_controller) (Variables|Default|GetTracking%20MC))
    (Variables|Default|SetbIsTracking false)
    (Variables|Default|SetbIsReturning (Variables|Default|GetbAutoReturn))))

(event Custom|ToggleEnable
  (params (bEnabled :type Boolean))
  (Variables|Default|SetbEnabled bEnabled))

(event Custom|SetBaseColor
  (params (Color :type Linear%20Color%20Structure))
  (bind _output_get (Variables|Default|SetBaseColor Color))
  (Rendering|Material|SetVectorParameterValue (Variables|Default|GetMI%20Button) "Color" _output_get :!class /Script/Engine.MaterialInstanceDynamic))

(event Custom|Fully%20Pressed
  (Default|CallOnButtonFullyPressed self)
  (CallFunction|ToggleGlowing true)
  (Variables|Default|SetbIsTracking false)
  (Variables|Default|SetbIsReturning false))

(event Custom|SetEmission
  (params (Strength :type Float%20%28single-precision%29))
  (Rendering|Material|SetScalarParameterValue (Variables|Default|GetMI%20Button) "Glow" Strength :!class /Script/Engine.MaterialInstanceDynamic))

(event Custom|ToggleGlowing
  (params (bEnabled :type Boolean))
  (Rendering|Material|SetScalarParameterValue (Variables|Default|GetMI%20Button) "Glow" (select bEnabled (Variables|Default|GetGlowing) 1.0) :!class /Script/Engine.MaterialInstanceDynamic))

(event EventBeginPlay)

(event EventTick
  (params (DeltaSeconds :type Float%20%28single-precision%29))
  (bind _vr_button (Variables|Default|GetVR_Button))
  (if (Variables|Default|GetbIsTracking)
    (bind _output_get (Variables|Default|SetCurrent%20Travel (Math|Float|Clamp(Float) (Math|Float|Absolute(Float) (Math|Vector|VectorLength (Math|Vector|ProjectVectorontoVector (- (Transformation|GetWorldLocation (Variables|Default|GetTracking%20MC)) (Variables|Default|GetMC%20intial%20Location)) (Math|Vector|GetUpVector (Variables|Default|GetVR_Button))))) 0.0 (Variables|Default|GetMaximum%20Travel))))
    (Development|PrintString (Utilities|String|ToString(Float) _output_get))
    (bind _output_get_2 (Variables|Default|SetButton%20Current%20Location (- (Variables|Default|GetButton%20initial%20Location) (* (Math|Vector|GetUpVector _vr_button) (Variables|Default|GetCurrent%20Travel)))))
    (Transformation|SetWorldLocation _vr_button _output_get_2 false false)
    (if (>= (Variables|Default|GetCurrent%20Travel) (Variables|Default|GetMaximum%20Travel))
      (if (Variables|Default|GetbEnabled)
        (CallFunction|FullyPressed)))
    (elif (Variables|Default|GetbIsReturning)
      (bind _output_get_3 (Variables|Default|SetButton%20Current%20Location (Math|Interpolation|VInterpTo (Variables|Default|GetButton%20Current%20Location) (Variables|Default|GetButton%20initial%20Location) (Utilities|Time|GetWorldDeltaSeconds) (Variables|Default|GetSpeedReturn))))
      (Transformation|SetWorldLocation (Variables|Default|GetVR_Button) _output_get_3 false false)
      (if (Class|KismetMathLibrary|EqualExactlyVectorVector (Variables|Default|GetButton%20initial%20Location) (Variables|Default|GetButton%20Current%20Location))
        (Variables|Default|SetbIsReturning false)
        (CallFunction|ToggleGlowing false)))))

(fn ConstructionScript
  (bind _returnvalue (Rendering|Material|CreateDynamicMaterialInstance (Variables|Default|GetVR_Button) 0 "/Game/Button/Button.Button" "None" :!class /Script/Engine.PrimitiveComponent))
  (Variables|Default|SetMI%20Button _returnvalue)
  (CallFunction|SetBaseColor (Variables|Default|GetBaseColor)))